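; BP_Obstacle is an endless runner obstacle that ends the run when the player pawn overlaps it.
; An overlap on its static mesh notifies the BP_ERun_PawnBase of the hit, then calls game over on the level manager if one is found.
; The construction script gives the mesh a random uniform scale, and a getter and setter store a parent reference.
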(event OnComponentBeginOverlap(StaticMesh)
  (params (OverlappedComponent :type Primitive%20Component%20Object%20Reference) (OtherActor :type Actor%20Object%20Reference) (OtherComp :type Primitive%20Component%20Object%20Reference) (OtherBodyIndex :type Integer) (bFromSweep :type Boolean) (SweepResult :type Hit%20Result%20Structure%20%28by%20ref%29))
  (bind (_levelmanager _levelmanagerfound) (CallFunction|GetLevelManager))
  (bind _asbp_erun_pawn_base (Utilities|Casting|CastToBP_ERun_PawnBase OtherActor))
  (Default|ERunHitObstacle _asbp_erun_pawn_base)
  (if _levelmanagerfound
    (Default|ERunGameOver _levelmanager)))

(fn ConstructionScript
  (Transformation|SetWorldScale3D (Variables|Default|GetStaticMesh) (Math|Conversions|ToVector(Float) (* 1.0 (Math|Random|RandomFloatinRange 1.0 2.0)))))

(fn ReturnParent
  (return (Variables|Default|GetParentRef)))

(fn SetParent
  (params (Parent :type BP%20E%20Run%20Spawner%20Base%20Object%20Reference))
  (Variables|Default|SetParentRef Parent)
  (return false))