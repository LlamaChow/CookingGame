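; Actor component for the endless runner that scrolls its owning actor at the level's lane speed.
; BeginPlay caches the level manager if one is found, and Tick reads its LaneSpeed every frame without a validity check.
; The owner's world forward vector, scaled by speed and delta time, is applied as a local offset without sweep, so the owner's rotation affects the direction twice.
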(event EventTick
  (params (DeltaSeconds :type Float%20%28single-precision%29))
  (Variables|Default|SetDeltaSeconds DeltaSeconds)
  (bind _output_get (Variables|Default|SetMovement (* (* (Transformation|GetActorForwardVector (Components|GetOwner)) (Variables|/Game/Blueprints/BP_LevelManager.BP_LevelManager_C|GetLaneSpeed (Variables|Default|GetLevelManagerRef))) (Variables|Default|GetDeltaSeconds))))
  (Transformation|AddActorLocalOffset (Components|GetOwner) _output_get false false))

(event EventBeginPlay
  (bind (_levelmanager _levelmanagerfound) (CallFunction|GetLevelManager))
  (if _levelmanagerfound
    (Variables|Default|SetLevelManagerRef _levelmanager)))