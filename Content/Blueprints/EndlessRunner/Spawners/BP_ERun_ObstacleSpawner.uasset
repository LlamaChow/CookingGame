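; Endless runner obstacle spawner that places obstacles at its own location at random intervals.
; On BeginPlay it finds the level manager, then waits a random delay between min and max, spawns through its parent spawner class, and repeats while the level is playing.
; Spawned obstacles that hit the bounds are destroyed after the parent handler runs.
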(event Custom|LineUpNextObstacleSpawn
  (Utilities|FlowControl|Delay (Math|Random|RandomFloatinRange (Variables|Default|GetMinDelay) (Variables|Default|GetMaxDelay)))
  (CallFunction|PlaceObstacle)
  (if (Variables|/Game/Blueprints/EndlessRunner/BP_Erun_LevelManager.BP_Erun_LevelManager_C|GetIsPlaying (Variables|Default|GetLevelManagerRef))
    (CallFunction|LineUpNextObstacleSpawn)))

(event EventBeginPlay
  (bind (_levelmanager _levelmanagerfound) (CallFunction|GetLevelManager))
  (if _levelmanagerfound
    (Variables|Default|SetLevelManagerRef _levelmanager)
    (Utilities|FlowControl|Delay 0.01)
    (CallFunction|LineUpNextObstacleSpawn)))

(fn ConstructionScript
  (|CallParentFunction))

(fn PlaceObstacle
  (bind _returnvalue (CallFunction|SpawnActor))
  (Transformation|SetActorLocation _returnvalue (Transformation|GetActorLocation) false false))

(fn SpawnActor
  (bind _returnvalue (|CallParentFunction))
  (return _returnvalue))

(fn SpawnedActorHitBounds
  (params (OutOfBoundsActor :type Actor%20Object%20Reference))
  (|CallParentFunction OutOfBoundsActor)
  (Actor|DestroyActor OutOfBoundsActor))