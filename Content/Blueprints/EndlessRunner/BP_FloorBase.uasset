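; BP_FloorBase is a floor Blueprint for the endless runner that moves itself at the lane speed set by the level manager.
; On BeginPlay it caches a valid level manager reference.
; Each Tick it scales its forward vector by that manager's LaneSpeed and delta time, then applies the result as a local-space offset without sweep.
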(event EventBeginPlay
  (bind _output (Utilities|GetLevelManager)
    (:Is%20Valid
      (Variables|Default|SetLevelManagerRef _output))))

(event EventTick
  (params (DeltaSeconds :type Float%20%28single-precision%29))
  (Variables|Default|SetDeltaSeconds DeltaSeconds)
  (bind _output_get (Variables|Default|SetMovement (* (* (Transformation|GetActorForwardVector) (Variables|/Game/Blueprints/BP_LevelManager.BP_LevelManager_C|GetLaneSpeed (Variables|Default|GetLevelManagerRef))) (Variables|Default|GetDeltaSeconds))))
  (Transformation|AddActorLocalOffset _output_get false false))

(fn ConstructionScript)