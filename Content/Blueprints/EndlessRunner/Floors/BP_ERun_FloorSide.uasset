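; BP_ERun_FloorSide is an endless runner floor side piece that fills a box area with randomly scattered meshes.
; Its construction script moves an instanced static mesh component to the box's relative location, used as a world position, then rebuilds its instances.
; Each instance gets a random point within the box bounds, random X and Y scales from MinXY to MaxXY, and an independently randomized height scale.
; The event graph has no active logic.
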(event EventBeginPlay
  (|CallParentFunction) ; This node is disabled and will not be called.\nDrag off pins to build functionality.
)

(event Collision|EventActorBeginOverlap
  (params (OtherActor :type Actor%20Object%20Reference)))

(event EventTick
  (params (DeltaSeconds :type Float%20%28single-precision%29)))

(fn ConstructionScript
  (bind _box (Variables|Default|GetBox))
  (bind _minxy (Variables|Default|GetMinXY))
  (bind _maxxy (Variables|Default|GetMaxXY))
  (bind (_origin _boxextent) (Collision|GetComponentBounds _box))
  (|CallParentFunction)
  (Transformation|SetWorldLocation (Variables|Default|GetInstancedStaticMesh) (Variables|/Script/Engine.SceneComponent|GetRelativeLocation (Variables|Default|GetBox)) false false)
  (Components|InstancedStaticMesh|ClearInstances (Variables|Default|GetInstancedStaticMesh))
  (for _index (range 0 10)
    (Components|InstancedStaticMesh|AddInstance (Variables|Default|GetInstancedStaticMesh) (Math|Transform|MakeTransform (Math|Random|RandomPointinBoundingBox _origin _boxextent) "0, 0, 0" (Math|Vector|MakeVector (Math|Random|RandomFloatinRange _minxy _maxxy) (Math|Random|RandomFloatinRange _minxy _maxxy) (Math|Random|RandomFloatinRange 2.0 2e+01))) false)))