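; BP_IntrctMGame is an interactable that opens a minigame UI when E is pressed within range.
; A Sphere overlap sets the IsInRange flag and shows the Widget component; end overlap clears the flag but also sets the Widget visible.
; While in range, each E press creates a new WBP_MiniGame, adds it to the viewport and shows the mouse cursor.
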(event OnComponentBeginOverlap(Sphere)
  (params (OverlappedComponent :type Primitive%20Component%20Object%20Reference) (OtherActor :type Actor%20Object%20Reference) (OtherComp :type Primitive%20Component%20Object%20Reference) (OtherBodyIndex :type Integer) (bFromSweep :type Boolean) (SweepResult :type Hit%20Result%20Structure%20%28by%20ref%29))
  (Rendering|SetVisibility (Variables|Default|GetWidget) true false)
  (Variables|Default|SetIsInRange true))

(event OnComponentEndOverlap(Sphere)
  (params (OverlappedComponent :type Primitive%20Component%20Object%20Reference) (OtherActor :type Actor%20Object%20Reference) (OtherComp :type Primitive%20Component%20Object%20Reference) (OtherBodyIndex :type Integer))
  (Rendering|SetVisibility (Variables|Default|GetWidget) true false)
  (Variables|Default|SetIsInRange false))

(event Input|KeyboardEvents|E
  (params (Key :type Key%20Structure :default "None"))
  (:Pressed
    (if (Variables|Default|GetIsInRange)
      (bind _returnvalue (UserInterface|CreateWidget "/Game/Blueprints/WidgetBlueprints/Pages/WBP_MiniGame.WBP_MiniGame_C"))
      (UserInterface|Viewport|AddtoViewport _returnvalue 0)
      (Variables|/Script/Engine.PlayerController|SetbShowMouseCursor (Game|GetPlayerController 0) true))))

(fn ConstructionScript
  (|CallParentFunction))